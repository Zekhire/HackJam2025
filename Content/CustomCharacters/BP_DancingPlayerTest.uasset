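; BP_DancingPlayerTest is a test Blueprint, named for a dancing player, that checks gamepad face button input through Enhanced Input.
; On BeginPlay it adds the IM_Gamepad mapping context to the first player controller's input subsystem.
; The IA_X, IA_Y, IA_A and IA_B input actions each print their button letter, and no other logic is implemented.
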(event Input|EnhancedActionEvents|EnhancedInputActionIA_X
  (params (ActionValue :type Boolean) (ElapsedSeconds :type Float%20%28double-precision%29) (TriggeredSeconds :type Float%20%28double-precision%29) (InputAction :type Input%20Action%20Object%20Reference :default "/Game/InputMapping/IA_X.IA_X"))
  (Development|PrintString "X"))

(event Input|EnhancedActionEvents|EnhancedInputActionIA_Y
  (params (ActionValue :type Boolean) (ElapsedSeconds :type Float%20%28double-precision%29) (TriggeredSeconds :type Float%20%28double-precision%29) (InputAction :type Input%20Action%20Object%20Reference :default "/Game/InputMapping/IA_Y.IA_Y"))
  (Development|PrintString "Y"))

(event Input|EnhancedActionEvents|EnhancedInputActionIA_B
  (params (ActionValue :type Boolean) (ElapsedSeconds :type Float%20%28double-precision%29) (TriggeredSeconds :type Float%20%28double-precision%29) (InputAction :type Input%20Action%20Object%20Reference :default "/Game/InputMapping/IA_B.IA_B"))
  (Development|PrintString "B"))

(event Input|EnhancedActionEvents|EnhancedInputActionIA_A
  (params (ActionValue :type Boolean) (ElapsedSeconds :type Float%20%28double-precision%29) (TriggeredSeconds :type Float%20%28double-precision%29) (InputAction :type Input%20Action%20Object%20Reference :default "/Game/InputMapping/IA_A.IA_A"))
  (Development|PrintString "A"))

(event EventBeginPlay
  (Input|AddMappingContext (PlayerController|LocalPlayerSubsystems|GetEnhancedInputLocalPlayerSubsystem (Game|GetPlayerController 0)) "/Game/InputMapping/IM_Gamepad.IM_Gamepad" 0 "(bIgnoreAllPressedKeysUntilRelease=True,bForceImmediately=False,bNotifyUserSettings=False)"))

(event Collision|EventActorBeginOverlap
  (params (OtherActor :type Actor%20Object%20Reference)))

(event EventTick
  (params (DeltaSeconds :type Float%20%28single-precision%29)))

(fn ConstructionScript)