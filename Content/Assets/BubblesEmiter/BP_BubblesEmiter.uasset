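; BP_BubblesEmiter is an emitter actor that periodically spawns BP_Bullet bubbles around itself.
; Tick constructs a BP_BubbleTracker behaviour for PlayerBubble every frame, while an accumulated timer triggers spawning once each PeriodS.
; SpawnBullet places the bullet at a random angle on a fixed-radius circle in the emitter's world YZ plane, passes it the tracker, and assigns a random type indexed by ButtonSymbols length.
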(event EventBeginPlay)

(event Collision|EventActorBeginOverlap
  (params (OtherActor :type Actor%20Object%20Reference)))

(event EventTick
  (params (DeltaSeconds :type Float%20%28single-precision%29))
  (bind _returnvalue (Game|ConstructObjectfromClass "/Game/Assets/BubblesEmiter/BulletBehaviours/BP_BubbleTracker.BP_BubbleTracker_C" (Variables|Default|GetPlayerBubble)))
  (bind _spawn (CallFunction|SpawnCounterAcc DeltaSeconds))
  (if _spawn
    (CallFunction|SpawnBullet 500 0 _returnvalue)))

(fn ConstructionScript)

(fn SpawnBullet
  (params (Radius :type Integer) (Speed :type Integer) (BulletBehaviourIn :type BP%20I%20Bullet%20Behaviour%20Object%20Reference))
  (bind _returnvalue (Transformation|GetActorTransform))
  (LocalVariables|SetBulletBehaviour BulletBehaviourIn)
  (LocalVariables|SetRadius_ (Math|Conversions|ToFloat(Integer) Radius))
  (LocalVariables|SetSpeed_ (Math|Conversions|ToFloat(Integer) Speed))
  (LocalVariables|SetAzimuthalAngle 0.0)
  (LocalVariables|SetPolarAngle (* (* (LocalVariables|GetPI) 2.0) (Math|Random|RandomFloat)))
  (Utilities|FlowControl|Sequence
    (:then_0
      (bind _output_get (LocalVariables|SetxCoord (- (.x (.location _returnvalue)) 0.0))))
    (:then_1
      (bind _output_get_2 (LocalVariables|SetyCoord (- (.y (.location _returnvalue)) (* (* (LocalVariables|GetRadius_) (Math|Trig|Sin(Radians) (LocalVariables|GetPolarAngle))) 1.0)))))
    (:then_2
      (bind _output_get_3 (LocalVariables|SetzCoord (- (.z (.location _returnvalue)) (* (* (LocalVariables|GetRadius_) (Math|Trig|Cos(Radians) (LocalVariables|GetPolarAngle))) 1.0))))
      (bind _returnvalue_2 (Game|SpawnActorfromClass "/Game/Assets/BubblesEmiter/BP_Bullet.BP_Bullet_C" (Math|Transform|MakeTransform (Math|Vector|MakeVector _output_get _output_get_2 _output_get_3) "0, 0, 0" (Math|Conversions|ToVector(Float) (Variables|Default|GetScale))) "Undefined" "MultiplyWithRoot" 0 (LocalVariables|GetBulletBehaviour) 0))
      (Default|ChangeType _returnvalue_2 (Math|Random|RandomInteger (Utilities|Map|Length (Variables|Default|GetButtonSymbols))))
      (return _returnvalue_2))))

(fn SpawnCounterAcc
  (params (DeltaTime :type Float%20%28double-precision%29))
  (bind _output_get (Variables|Default|SetCounterS (+ DeltaTime (Variables|Default|GetCounterS))))
  (if (>= _output_get (Variables|Default|GetPeriodS))
    (Variables|Default|SetCounterS 0.0)
    (return true)
    (else
      (return false))))