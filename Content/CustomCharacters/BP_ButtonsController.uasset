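; Button controller that judges player button presses against the incoming bullet bubbles, driving score and combo.
; CheckButtonType tests only the front of the bullets queue, requiring it to be in the player's bubble range and match the pressed type.
; A hit destroys that bubble through BP_BubbleTracker and calls AddScoreCall on BP_EventManager.
; An empty queue, out-of-range bullet or wrong type calls BreakComboCall instead.
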(event Custom|CheckButtonType
  (params (ButtonType :type Integer))
  (bind _bulletscontroller (Variables|Default|GetBulletsController))
  (bind _bulletsqueuecontroller (Variables|/Game/Assets/BubblesEmiter/BP_BulletsController.BP_BulletsController_C|GetBulletsQueueController _bulletscontroller))
  (bind _bulletsqueue (Variables|/Game/Assets/BubblesEmiter/BP_BulletsQueueController.BP_BulletsQueueController_C|GetBulletsQueue _bulletsqueuecontroller))
  (bind _output (Utilities|Array|Get(acopy) _bulletsqueue))
  (bind _bulletbehaviour (Variables|/Game/Assets/BubblesEmiter/BP_Bullet.BP_Bullet_C|GetBulletBehaviour _output))
  (if (> (Utilities|Array|Length _bulletsqueue) 0)
    (if (Variables|/Game/Assets/BubblesEmiter/BulletBehaviours/BP_IBulletBehaviour.BP_IBulletBehaviour_C|GetInPlayerBubbleRange _bulletbehaviour)
      (if (== ButtonType (Variables|/Game/Assets/BubblesEmiter/BP_Bullet.BP_Bullet_C|GetType _output))
        (bind _asbp_bubble_tracker (Utilities|Casting|CastToBP_BubbleTracker _bulletbehaviour))
        (Default|BehaviourtoDestroy _asbp_bubble_tracker)
        (bind _eventmanager (CallFunction|GetEventManager))
        (Default|AddScoreCall _eventmanager)
        (else
          (bind _eventmanager_2 (CallFunction|GetEventManager :!label _label))
          (Default|BreakComboCall _eventmanager_2)))
      (else
        (goto _label)))
    (else
      (goto _label))))

(event EventBeginPlay)

(event EventTick
  (params (DeltaSeconds :type Float%20%28single-precision%29)))

(fn GetEventManager
  (bind _returnvalue (Actor|GetActorOfClass "/Game/Assets/EventManager/BP_EventManager.BP_EventManager_C"))
  (return _returnvalue))