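; BP_EventManager is a broadcast hub that relays game events for scoring, a dancing player and audio playback to interested actors.
; Each custom event finds all actors implementing the matching interface (BPI_ScoreEvents, BPI_DancingPlayer or BPI_AudioDataUser) and sends each the corresponding message.
; It covers combo breaks, score additions, player falls, audio sample data with progress, and audio end.
; Receivers are looked up afresh on every call, including each audio sample callback, rather than cached.
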(event Custom|AudioSamplesCallback
  (params (Samples :type Array%20of%20Floats%20%28double-precision%29) (Progress :type Float%20%28double-precision%29))
  (bind _outactors (Actor|GetAllActorswithInterface "/Game/Assets/EventManager/BPI_AudioDataUser.BPI_AudioDataUser_C"))
  (for _array_element _outactors
    (Class|BPIAudioDataUser|AudioSamplesCallback(Message) _array_element Samples Progress)))

(event Custom|BreakComboCall
  (bind _outactors (Actor|GetAllActorswithInterface "/Game/Assets/EventManager/BPI_ScoreEvents.BPI_ScoreEvents_C"))
  (for _array_element _outactors
    (Class|BPIScoreEvents|BreakCombo(Message) _array_element)))

(event Custom|FallPlayerCall
  (bind _outactors (Actor|GetAllActorswithInterface "/Game/CustomCharacters/BPI_DancingPlayer.BPI_DancingPlayer_C"))
  (for _array_element _outactors
    (Class|BPIDancingPlayer|Fall(Message) _array_element)))

(event Custom|AddScoreCall
  (bind _outactors (Actor|GetAllActorswithInterface "/Game/Assets/EventManager/BPI_ScoreEvents.BPI_ScoreEvents_C"))
  (for _array_element _outactors
    (Class|BPIScoreEvents|AddScore(Message) _array_element)))

(event Custom|AudioEndedCallback
  (bind _outactors (Actor|GetAllActorswithInterface "/Game/Assets/EventManager/BPI_AudioDataUser.BPI_AudioDataUser_C"))
  (for _array_element _outactors
    (Class|BPIAudioDataUser|AudioEndedCallback(Message) _array_element)))

(event EventBeginPlay)

(event Collision|EventActorBeginOverlap
  (params (OtherActor :type Actor%20Object%20Reference)))

(event EventTick
  (params (DeltaSeconds :type Float%20%28single-precision%29)))

(fn ConstructionScript)