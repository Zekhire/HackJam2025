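; BP_ProgressBar is an actor that scales a bar mesh to show progress reported by an audio samples callback.
; On BeginPlay it computes a full length from sample count, sample scale and offset.
; Each AudioSamplesCallback passes Progress to ProgressBarUpdate, which sets the bar's Y world scale proportional to that length, reusing its relative X and Z scale.
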(event EventBeginPlay
  (Utilities|FlowControl|Sequence
    (:then_0
      (Variables|Default|SetFullScale (* (Variables|Default|GetSamplesAmount) (+ (Variables|Default|GetsampleScale) (Variables|Default|GetsamplesOffset)))))))

(event Collision|EventActorBeginOverlap
  (params (OtherActor :type Actor%20Object%20Reference)))

(event EventTick
  (params (DeltaSeconds :type Float%20%28single-precision%29)))

(event EventAudioSamplesCallback
  (params (Samples :type Array%20of%20Floats%20%28double-precision%29) (Progress :type Float%20%28double-precision%29))
  (CallFunction|ProgressBarUpdate Progress))

(fn ConstructionScript)

(fn ProgressBarUpdate
  (params (Progress :type Float%20%28double-precision%29))
  (bind _progressbar (Variables|Default|Getprogressbar))
  (bind _relativescale3d (Variables|/Script/Engine.SceneComponent|GetRelativeScale3D _progressbar))
  (Transformation|SetWorldScale3D _progressbar (Math|Vector|MakeVector (.x _relativescale3d) (* Progress (Variables|Default|GetFullScale) 0.05 0.25 0.8) (.z _relativescale3d))))