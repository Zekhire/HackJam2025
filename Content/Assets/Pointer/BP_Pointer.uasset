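; BP_Pointer is a pointer actor that tracks which BP_Bullet actors currently overlap it.
; Begin and end overlap events cast the other actor to BP_Bullet and add it to or remove it from the OverlappedBullets array.
; CheckIfPointerOverlapWithBullet searches that array to report whether a given bullet is under the pointer, so the check runs without a new overlap query.
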(event EventBeginPlay)

(event Collision|EventActorBeginOverlap
  (params (OtherActor :type Actor%20Object%20Reference))
  (bind _asbp_bullet (Utilities|Casting|CastToBP_Bullet OtherActor))
  (Utilities|Array|Add (Variables|Default|GetOverlappedBullets) _asbp_bullet))

(event EventTick
  (params (DeltaSeconds :type Float%20%28single-precision%29)))

(event Collision|EventActorEndOverlap
  (params (OtherActor :type Actor%20Object%20Reference))
  (bind _asbp_bullet (Utilities|Casting|CastToBP_Bullet OtherActor))
  (Utilities|Array|RemoveItem (Variables|Default|GetOverlappedBullets) _asbp_bullet))

(fn ConstructionScript)

(fn CheckifPointerOverlapwithBullet
  (params (Bullet :type BP%20Bullet%20Object%20Reference))
  (return (>= (Utilities|Array|FindItem (Variables|Default|GetOverlappedBullets) Bullet) 0)))