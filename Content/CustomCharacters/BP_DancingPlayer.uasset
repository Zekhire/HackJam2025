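; BP_DancingPlayer is the player character of a rhythm-style game, dancing in place and reacting to gamepad button presses.
; PreparePlayer adds input mapping and links the bullets and score controllers to BPButtonsController, which checks face-button presses.
; Random dance montages loop, speeding up with combo up to a cap.
; Fall interrupts dancing and blocks buttons, then grants brief invulnerability, while the left stick shows and rotates a pointer actor.
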(event Custom|Dance
  (if (not (Variables|Default|GetisFalling)) :!label _label
    (Animation|Montage|PlayMontage (Variables|Character|GetMesh) (Utilities|Array|Get(acopy) (Variables|Default|GetDanceAnimations) (Math|Random|RandomInteger (Utilities|Array|Length (Variables|Default|GetDanceAnimations)))) (+ (Math|Float|Min(Float) (* (Variables|/Game/Assets/Score/BP_ScoreController.BP_ScoreController_C|GetCombo (Variables|Default|GetScoreController)) 0.4) (* 5.0 0.4)) 1.0)
      (:OnCompleted
        (goto _label)))))

(event Custom|PreparePlayer
  (bind _bp_buttonscontroller (Variables|Default|GetBP_ButtonsController))
  (Input|AddMappingContext (PlayerController|LocalPlayerSubsystems|GetEnhancedInputLocalPlayerSubsystem (Game|GetPlayerController 0)) "/Game/InputMapping/IM_Gamepad.IM_Gamepad" 0 "(bIgnoreAllPressedKeysUntilRelease=True,bForceImmediately=False,bNotifyUserSettings=False)")
  (bind _returnvalue (Actor|GetActorOfClass "/Game/Assets/BubblesEmiter/BP_BulletsController.BP_BulletsController_C"))
  (Variables|/Game/CustomCharacters/BP_ButtonsController.BP_ButtonsController_C|SetBulletsController _bp_buttonscontroller _returnvalue)
  (bind _returnvalue_2 (Actor|GetActorOfClass "/Game/Assets/Score/BP_ScoreController.BP_ScoreController_C"))
  (bind _output_get (Variables|Default|SetScoreController _returnvalue_2))
  (Variables|/Game/CustomCharacters/BP_ButtonsController.BP_ButtonsController_C|SetScoreController _bp_buttonscontroller _output_get)
  (CallFunction|Dance))

(event Input|EnhancedActionEvents|EnhancedInputActionIA_X
  (params (ActionValue :type Boolean) (ElapsedSeconds :type Float%20%28double-precision%29) (TriggeredSeconds :type Float%20%28double-precision%29) (InputAction :type Input%20Action%20Object%20Reference :default "/Game/InputMapping/IA_X.IA_X"))
  (if (not (Variables|Default|GetisFalling))
    (Default|CheckButtonType (Variables|Default|GetBP_ButtonsController))))

(event Input|EnhancedActionEvents|EnhancedInputActionIA_Y
  (params (ActionValue :type Boolean) (ElapsedSeconds :type Float%20%28double-precision%29) (TriggeredSeconds :type Float%20%28double-precision%29) (InputAction :type Input%20Action%20Object%20Reference :default "/Game/InputMapping/IA_Y.IA_Y"))
  (if (not (Variables|Default|GetisFalling))
    (Default|CheckButtonType (Variables|Default|GetBP_ButtonsController) 1)))

(event Input|EnhancedActionEvents|EnhancedInputActionIA_B
  (params (ActionValue :type Boolean) (ElapsedSeconds :type Float%20%28double-precision%29) (TriggeredSeconds :type Float%20%28double-precision%29) (InputAction :type Input%20Action%20Object%20Reference :default "/Game/InputMapping/IA_B.IA_B"))
  (if (not (Variables|Default|GetisFalling))
    (Default|CheckButtonType (Variables|Default|GetBP_ButtonsController) 3)))

(event Input|EnhancedActionEvents|EnhancedInputActionIA_A
  (params (ActionValue :type Boolean) (ElapsedSeconds :type Float%20%28double-precision%29) (TriggeredSeconds :type Float%20%28double-precision%29) (InputAction :type Input%20Action%20Object%20Reference :default "/Game/InputMapping/IA_A.IA_A"))
  (if (not (Variables|Default|GetisFalling))
    (Default|CheckButtonType (Variables|Default|GetBP_ButtonsController) 2)))

(event Input|EnhancedActionEvents|EnhancedInputActionIA_LAnalog
  (params (ActionValue :type Vector%202D%20Structure) (ElapsedSeconds :type Float%20%28double-precision%29) (TriggeredSeconds :type Float%20%28double-precision%29) (InputAction :type Input%20Action%20Object%20Reference :default "/Game/InputMapping/IA_LAnalog.IA_LAnalog"))
  (:Triggered
    (bind _returnvalue (Actor|GetActorOfClass "/Game/Assets/Pointer/BP_Pointer.BP_Pointer_C"))
    (Rendering|SetActorHiddenInGame _returnvalue false)
    (Transformation|SetActorRotation _returnvalue (Math|Rotator|MakeRotator (* (Class|KismetMathLibrary|DegAtan2 (.y ActionValue) (.x ActionValue)) -1.0) (.pitch (Transformation|GetActorRotation _returnvalue)) (.yaw (Transformation|GetActorRotation _returnvalue)))))
  (:Completed
    (bind _returnvalue_2 (Actor|GetActorOfClass "/Game/Assets/Pointer/BP_Pointer.BP_Pointer_C"))
    (Rendering|SetActorHiddenInGame _returnvalue_2 true)))

(event EventBeginPlay
  (Components|Animation|PlayAnimation (Variables|Character|GetMesh) "/Game/Animations/SadIdle_UE_Montage.SadIdle_UE_Montage" true))

(event Collision|EventActorBeginOverlap
  (params (OtherActor :type Actor%20Object%20Reference)))

(event EventTick
  (params (DeltaSeconds :type Float%20%28single-precision%29)))

(event EventFall
  (if (Variables|Default|GetisVulnerable)
    (if (not (Variables|Default|GetisFalling))
      (Variables|Default|SetisFalling true)
      (Variables|Default|SetisVulnerable false)
      (Animation|Montage|PlayMontage (Variables|Character|GetMesh) "/Game/Animations/FallingForwardDeath_UE_Montage.FallingForwardDeath_UE_Montage"
        (:OnCompleted
          (Variables|Default|SetisFalling false)
          (CallFunction|Dance)
          (Utilities|FlowControl|Delay 2.0)
          (Variables|Default|SetisVulnerable true))))))

(fn ConstructionScript)