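; BP_BubbleButton is a bubble button actor that displays a symbol matching its Type.
; On BeginPlay it caches its widget component's WB_ButtonSymbol instance and applies the current Type.
; ChangeType stores the new Type, looks up its texture in the ButtonSymbols map and sets it as the widget's image brush.
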(event EventBeginPlay
  (bind _aswb_button_symbol (Utilities|Casting|CastToWB_ButtonSymbol (UserInterface|GetWidget (Variables|Default|GetWidget))))
  (Variables|Default|SetButtonWidget _aswb_button_symbol)
  (CallFunction|ChangeType (Variables|Default|GetType)))

(event Collision|EventActorBeginOverlap
  (params (OtherActor :type Actor%20Object%20Reference)))

(event EventTick
  (params (DeltaSeconds :type Float%20%28single-precision%29)))

(fn ConstructionScript)

(fn ChangeType
  (params (Type :type Integer))
  (bind _output_get (Variables|Default|SetType Type))
  (Appearance|SetBrushfromTexture (Variables|/Game/Assets/BubblesEmiter/BubbleButton/WB_ButtonSymbol.WB_ButtonSymbol_C|GetImage_76 (Variables|Default|GetButtonWidget)) (.Value (Utilities|Map|Find (Variables|Default|GetButtonSymbols) _output_get)) false))