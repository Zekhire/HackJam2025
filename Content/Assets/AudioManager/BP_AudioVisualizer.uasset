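; BP_AudioVisualizer plays a sound and drives an audio spectrum display in sync with it.
; Each playback-percent callback updates BP_ProgressBar and converts the percent to elapsed seconds.
; It then samples precomputed Constant-Q NRT data at that time, setting BP_Spectrum's static mesh Z scales per band.
; Disconnected leftovers include a cooked-FFT readout, the only consumer of the generated frequency array, and BP_PlayerBubble scaling.
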(event Custom|PlaybackChange
  (params (PlayingSoundWave :type Sound%20Wave%20Object%20Reference) (PlaybackPercent :type Float%20%28single-precision%29))
  (bind _returnvalue (Actor|GetActorOfClass "/Game/Assets/AudioManager/BP_ProgressBar.BP_ProgressBar_C"))
  (Default|ProgressBarUpdate _returnvalue PlaybackPercent)
  (bind _output_get (Variables|Default|SetPlayedTime (* PlaybackPercent (Variables|Default|GetDuration))))
  (for (_array_element _array_index) (Class|ConstantQNRT|GetNormalizedChannelConstantQatTime (Variables|Default|GetConstantQNRTRef) _output_get)
    (Utilities|FlowControl|Sequence
      (:then_0
        (Transformation|SetRelativeScale3D (Utilities|Array|Get(acopy) (Actor|GetComponentsByClass (Variables|Default|GetSpectrum) "/Script/Engine.StaticMeshComponent") _array_index) (Math|Vector|MakeVector (.x (Variables|/Script/Engine.SceneComponent|GetRelativeScale3D (Utilities|Array|Get(acopy) (Actor|GetComponentsByClass (Variables|Default|GetSpectrum) "/Script/Engine.StaticMeshComponent") _array_index))) (.y (Variables|/Script/Engine.SceneComponent|GetRelativeScale3D (Utilities|Array|Get(acopy) (Actor|GetComponentsByClass (Variables|Default|GetSpectrum) "/Script/Engine.StaticMeshComponent") _array_index))) (* _array_element 0.2)))))))

(event EventBeginPlay
  (Utilities|FlowControl|Sequence
    (:then_0
      (bind _frequencies1 (CallFunction|GenerateFreqArray 0.0 5e+03 48))
      (Variables|Default|SetFrequenciesToGet _frequencies1)
      (bind _returnvalue (Actor|GetActorOfClass "/Game/Assets/AudioManager/BP_Spectrum.BP_Spectrum_C"))
      (Variables|Default|SetSpectrum _returnvalue))
    (:then_1
      (Audio|Components|Audio|SetSound (Variables|Default|GetAudio) (Variables|Default|GetSound))
      (Variables|Default|SetDuration (Variables|/Script/Engine.SoundBase|GetDuration (Variables|Default|GetSound)))
      (EventDispatchers|BindEventtoOnAudioPlaybackPercent (Variables|Default|GetAudio) (delegate Custom|PlaybackChange))
      (Audio|Components|Audio|Play (Variables|Default|GetAudio) 0.0))))

(event Collision|EventActorBeginOverlap
  (params (OtherActor :type Actor%20Object%20Reference)))

(event EventTick
  (params (DeltaSeconds :type Float%20%28single-precision%29)))

(fn ConstructionScript)

(fn GenerateFreqArray
  (params (MinFreq :type Float%20%28double-precision%29) (MaxFreq :type Float%20%28double-precision%29) (Amount :type Integer))
  (for _index (range 0 (- Amount 1))
    (Utilities|Array|Add (LocalVariables|GetFrequencies) (Math|Float|Lerp MinFreq MaxFreq (/ _index (Math|Conversions|ToFloat(Integer) Amount)))))
  (return (LocalVariables|GetFrequencies)))