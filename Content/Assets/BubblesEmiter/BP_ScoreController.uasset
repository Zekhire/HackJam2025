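; Score controller Blueprint in the bubble emitter assets that tracks Score and a Combo count.
; Its AddPoints event awards points that grow with each consecutive combo step up to a fixed cap, then increments Combo and prints the new Score.
; Nothing in this Blueprint resets Combo or calls AddPoints, and its default events are empty.
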(event Custom|AddPoints
  (Utilities|FlowControl|Sequence
    (:then_0
      (if (< (+ (Variables|Default|GetCombo) 1) 5)
        (Variables|Default|SetScore (+ (Variables|Default|GetScore) (* 10 (+ (Variables|Default|GetCombo) 1))))
        (else
          (Variables|Default|SetScore (+ (Variables|Default|GetScore) 50)))))
    (:then_1
      (Variables|Default|SetCombo (+ (Variables|Default|GetCombo) 1)))
    (:then_2
      (Development|PrintString (Utilities|String|ToString(Integer) (Variables|Default|GetScore))))))

(event EventBeginPlay)

(event Collision|EventActorBeginOverlap
  (params (OtherActor :type Actor%20Object%20Reference)))

(event EventTick
  (params (DeltaSeconds :type Float%20%28single-precision%29)))

(fn ConstructionScript)