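; Bullet behaviour for a tracker bubble that homes in on the player's bubble.
; Each update lerps the bullet toward the player bubble by SpeedAlpha, independent of DeltaTime, and shows its Sphere1 while in range.
; Progress is normalized from spawn distance and both radii.
; At 1 or above, it breaks the combo, removes the bullet from the controller's queue and destroys it.
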(fn Behaviour
  (params (DeltaTime :type Float%20%28double-precision%29))
  (|CallParentFunction DeltaTime)
  (Utilities|FlowControl|Sequence
    (:then_0
      (CallFunction|BulletMove))
    (:then_1
      (if (Variables|Default|GetInPlayerBubbleRange)
        (CallFunction|BehaviourifinPlayerBubble DeltaTime)))
    (:then_2
      (bind _normalizeddistanceout (CallFunction|GetNormalizedDistancefromPlayerBubble))
      (if (>= _normalizeddistanceout 1.0)
        (bind _eventmanager (Default|GetEventManager (Variables|Default|GetBullet)))
        (Default|BreakComboCall _eventmanager)
        (CallFunction|BehaviourtoDestroy)))))

(fn BehaviourifinPlayerBubble
  (params (DeltaTime :type Float%20%28double-precision%29))
  (|CallParentFunction DeltaTime)
  (Rendering|SetVisibility (Variables|/Game/Assets/BubblesEmiter/BP_Bullet.BP_Bullet_C|GetSphere1 (Variables|Default|GetBullet)) true false))

(fn GetNormalizedDistancefromPlayerBubble
  (bind _playerbubble (Variables|Default|GetPlayerBubble))
  (bind _bullet (Variables|Default|GetBullet))
  (bind _returnvalue (Transformation|GetActorTransform _playerbubble))
  (bind _initialtransform (Variables|/Game/Assets/BubblesEmiter/BP_Bullet.BP_Bullet_C|GetInitialTransform _bullet))
  (bind _returnvalue_2 (Math|Transform|TransformLocation _returnvalue "0, 0, 0"))
  (bind _returnvalue_3 (Math|Transform|TransformLocation _initialtransform "0, 0, 0"))
  (bind _returnvalue_4 (Math|Vector|Distance(Vector) _returnvalue_2 _returnvalue_3))
  (bind _radius (Default|GetRadius (Variables|Default|GetPlayerBubble)))
  (bind _radius_2 (Default|GetRadius (Variables|Default|GetBullet)))
  (LocalVariables|SetRadiusDiff (- _radius _radius_2))
  (bind _output_get (LocalVariables|SetNormalizedDistance (/ (- _returnvalue_4 (- (Math|Vector|Distance(Vector) _returnvalue_2 (Math|Transform|TransformLocation (Transformation|GetActorTransform (Variables|Default|GetBullet)) "0, 0, 0")) (LocalVariables|GetRadiusDiff))) (- _returnvalue_4 (LocalVariables|GetRadiusDiff)))))
  (return _output_get))

(fn BulletMove
  (bind _bullet (Variables|Default|GetBullet))
  (bind _bullet_2 (Variables|Default|GetBullet))
  (bind _returnvalue (Transformation|GetActorTransform _bullet))
  (Transformation|SetActorTransform _bullet_2 (Math|Transform|MakeTransform (Math|Vector|Lerp(Vector) (Math|Transform|TransformLocation (Transformation|GetActorTransform _bullet_2) "0, 0, 0") (Math|Transform|TransformLocation (Transformation|GetActorTransform (Variables|Default|GetPlayerBubble)) "0, 0, 0") (Variables|Default|GetSpeedAlpha)) (.rotation _returnvalue) (.scale _returnvalue))))

(fn BehaviourtoDestroy
  (bind _bullet (Variables|Default|GetBullet))
  (Utilities|Array|RemoveItem (Variables|/Game/Assets/BubblesEmiter/BP_BulletsQueueController.BP_BulletsQueueController_C|GetBulletsQueue (Variables|/Game/Assets/BubblesEmiter/BP_BulletsController.BP_BulletsController_C|GetBulletsQueueController (Variables|/Game/Assets/BubblesEmiter/BP_Bullet.BP_Bullet_C|GetBulletsController _bullet))) _bullet)
  (Actor|DestroyActor (Variables|Default|GetBullet)))