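; BP_Spectrum is an actor that builds the bars for a spectrum display, presumably for audio visualization.
; On BeginPlay it adds a row of cube mesh components along local Y, sized, spaced and counted by variables, each using the spectrum material.
; The bars start at zero Z scale and are stored in SpectrumSamplesArray; this graph contains no logic that animates them.
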(event EventBeginPlay
  (bind _samplescale (Variables|Default|GetsampleScale))
  (Utilities|FlowControl|Sequence
    (:then_1
      (for _index (range 0 (- (Variables|Default|GetSamplesAmount) 1))
        (bind _returnvalue (AddComponent|AddStaticMeshComponent false (Math|Transform|MakeTransform (Math|Vector|MakeVector 0.0 (Math|Conversions|ToFloat(Integer) (* _index (Variables|Default|GetsamplesOffset))) 0.0) "0, 0, 0" (Math|Vector|MakeVector _samplescale _samplescale 0.0))))
        (Components|StaticMesh|SetStaticMesh _returnvalue "/Game/LevelPrototyping/Meshes/SM_Cube.SM_Cube")
        (Rendering|Material|SetMaterial _returnvalue 0 "/Game/Assets/AudioManager/Materials/MI_SpectrumMaterial.MI_SpectrumMaterial")
        (Utilities|Array|Add (Variables|Default|GetSpectrumSamplesArray) 0)))))

(event Collision|EventActorBeginOverlap
  (params (OtherActor :type Actor%20Object%20Reference)))

(event EventTick
  (params (DeltaSeconds :type Float%20%28single-precision%29)))

(fn ConstructionScript)