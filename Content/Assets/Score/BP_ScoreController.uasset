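; BP_ScoreController is a score controller that tracks the player's score and combo streak and displays the score in a WPI_Score widget created on BeginPlay.
; AddPoints, also triggered through AddScore, awards points that grow with the combo up to a cap, increments the combo, then pushes the new score to the widget.
; BreakCombo resets the combo and calls FallPlayerCall on the BP_EventManager found via GetActorOfClass.
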(event Custom|AddPoints
  (Utilities|FlowControl|Sequence
    (:then_0
      (if (< (+ (Variables|Default|GetCombo) 1) 5)
        (Variables|Default|SetScore (+ (Variables|Default|GetScore) (* 10 (+ (Variables|Default|GetCombo) 1))))
        (else
          (Variables|Default|SetScore (+ (Variables|Default|GetScore) 50)))))
    (:then_1
      (Variables|Default|SetCombo (+ (Variables|Default|GetCombo) 1)))
    (:then_2
      (Default|UpdateScore (Variables|Default|GetScoreWidget) (Variables|Default|GetScore)))))

(event EventBeginPlay
  (bind _returnvalue (UserInterface|CreateWidget "/Game/Assets/Score/WPI_Score.WPI_Score_C"))
  (bind _output_get (Variables|Default|SetScoreWidget _returnvalue))
  (UserInterface|Viewport|AddtoViewport _output_get 0))

(event Collision|EventActorBeginOverlap
  (params (OtherActor :type Actor%20Object%20Reference)))

(event EventTick
  (params (DeltaSeconds :type Float%20%28single-precision%29)))

(event EventBreakCombo
  (Variables|Default|SetCombo 0)
  (bind _eventmanager (CallFunction|GetEventManager))
  (Default|FallPlayerCall _eventmanager))

(event EventAddScore
  (CallFunction|AddPoints))

(fn ConstructionScript)

(fn GetEventManager
  (bind _returnvalue (Actor|GetActorOfClass "/Game/Assets/EventManager/BP_EventManager.BP_EventManager_C"))
  (return _returnvalue))