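; BP_Bullet is a bubble bullet actor that displays a button symbol matching its Type on a widget.
; On BeginPlay it sets that symbol, registers with the BulletsController's queue, links itself to its BulletBehaviour and stores its initial transform.
; Tick and sphere overlap-begin are delegated to BulletBehaviour, keeping movement or reaction logic outside the actor.
; GetRadius returns the radius scaled by the actor's X scale.
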(event OnComponentBeginOverlap(Sphere)
  (params (OverlappedComponent :type Primitive%20Component%20Object%20Reference) (OtherActor :type Actor%20Object%20Reference) (OtherComp :type Primitive%20Component%20Object%20Reference) (OtherBodyIndex :type Integer) (bFromSweep :type Boolean) (SweepResult :type Hit%20Result%20Structure%20%28by%20ref%29))
  (Default|OnPlayerBubbleEnter (Variables|Default|GetBulletBehaviour)))

(event OnComponentEndOverlap(Sphere)
  (params (OverlappedComponent :type Primitive%20Component%20Object%20Reference) (OtherActor :type Actor%20Object%20Reference) (OtherComp :type Primitive%20Component%20Object%20Reference) (OtherBodyIndex :type Integer)))

(event EventBeginPlay
  (Utilities|FlowControl|Sequence
    (:then_0
      (bind _aswb_button_symbol (Utilities|Casting|CastToWB_ButtonSymbol (UserInterface|GetWidget (Variables|Default|GetWidget))))
      (Variables|Default|SetButtonWidget _aswb_button_symbol)
      (CallFunction|ChangeType (Variables|Default|GetType))
      (Actor|GetActorOfClass "/Game/Assets/BubblesEmiter/BP_BulletsController.BP_BulletsController_C"))
    (:then_1
      (bind _returnvalue (Actor|GetActorOfClass "/Game/Assets/BubblesEmiter/BP_BulletsController.BP_BulletsController_C"))
      (Variables|Default|SetBulletsController _returnvalue)
      (Default|AddBullettoArray (Variables|/Game/Assets/BubblesEmiter/BP_BulletsController.BP_BulletsController_C|GetBulletsQueueController _returnvalue) self))
    (:then_2
      (Variables|/Game/Assets/BubblesEmiter/BulletBehaviours/BP_IBulletBehaviour.BP_IBulletBehaviour_C|SetBullet (Variables|Default|GetBulletBehaviour) self))
    (:then_3
      (Variables|Default|SetInitialTransform (Transformation|GetActorTransform)))))

(event Collision|EventActorBeginOverlap
  (params (OtherActor :type Actor%20Object%20Reference)))

(event EventTick
  (params (DeltaSeconds :type Float%20%28single-precision%29))
  (Default|Behaviour (Variables|Default|GetBulletBehaviour) DeltaSeconds))

(fn ConstructionScript)

(fn ChangeType
  (params (Type :type Integer))
  (bind _output_get (Variables|Default|SetType Type))
  (Appearance|SetBrushfromTexture (Variables|/Game/Assets/BubblesEmiter/BubbleButton/WB_ButtonSymbol.WB_ButtonSymbol_C|GetImage_76 (Variables|Default|GetButtonWidget)) (.Value (Utilities|Map|Find (Variables|Default|GetButtonSymbols) _output_get)) false))

(fn GetRadius
  (return (* (Variables|Default|GetRadius) (.x (.scale (Transformation|GetActorTransform))))))